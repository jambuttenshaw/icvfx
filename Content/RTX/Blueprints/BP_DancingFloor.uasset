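; BP_DancingFloor builds a grid of instanced mesh blocks with seeded random heights, forming an uneven floor.
; The construction script sizes the grid from Dimensions, Size and Height, storing each block's base location and random value.
; A sine-wave animation that would bob and stretch blocks through a batched transform update is left disconnected from Tick, so the floor stays static.
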(event EventBeginPlay)

(event Collision|EventActorBeginOverlap
  (params (OtherActor :type Actor%20Object%20Reference)))

(event EventTick
  (params (DeltaSeconds :type Float%20%28single-precision%29)))

(fn ConstructionScript
  (bind _dimensions (Variables|Default|GetDimensions))
  (bind _size (Variables|Default|GetSize))
  (bind _stream (Variables|Default|GetStream))
  (bind _height (Variables|Default|GetHeight))
  (bind _returnvalue (Math|Random|RandomFloatfromStream _stream))
  (bind _returnvalue_2 (* _returnvalue _height))
  (bind _returnvalue_3 (+ _returnvalue_2 1.0))
  (for _index (range 0 (Math|Float|Truncate (.x _dimensions)))
    (for _index_2 (range 0 (Math|Float|Truncate (.y _dimensions)))
      (Utilities|Array|Add (Variables|Default|Getinst_rnd) _returnvalue_3)
      (Utilities|Array|Add (Variables|Default|Getinst_init_loc) (Math|Vector|MakeVector (* _size _index) (* _size _index_2) 25.0))
      (Components|InstancedStaticMesh|AddInstance (Variables|Default|GetInstancedStaticMesh) (Math|Transform|MakeTransform (+ (Math|Vector|MakeVector (* _size _index) (* _size _index_2) 25.0) (Math|Vector|MakeVector 0.0 0.0 (* _returnvalue_3 25.0))) "0, 0, 0" (Math|Vector|MakeVector 1.0 1.0 _returnvalue_3)) false))))