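; BP_Lights is an actor that fills a box with randomly placed colored point lights, each paired with an instanced mesh.
; The construction script runs GenerateLights, which rebuilds the lights and ISMLights instances, drawing position, hue, source radius and intensity from a random stream.
; When Animate is on, Tick circles each light and its instance around the stored start position, at speeds varied by index.
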(event Custom|GenerateLights
  (bind _lightsradius (Variables|Default|GetLightsRadius))
  (bind _lightsintensity (Variables|Default|GetLightsIntensity))
  (bind _half_size (Variables|Default|GetHalf%20Size))
  (Components|InstancedStaticMesh|ClearInstances (Variables|Default|GetISM_Lights))
  (for _array_element (Variables|Default|GetLights)
    (Utilities|IsValid _array_element
      (:Is%20Valid
        (Components|DestroyComponent _array_element))))
  (Actor|Tick|SetActorTickEnabled (Variables|Default|GetAnimate))
  (for _index (range 0 (- (Variables|Default|GetCount) 1))
    (Utilities|Array|Add (Variables|Default|GetInitPos) (Class|KismetMathLibrary|RandomPointinBoundingBoxfromStream (Variables|Default|GetStream) _half_size _half_size))
    (bind _returnvalue (AddComponent|AddPointLightComponent false (Math|Transform|MakeTransform (Utilities|Array|Get(acopy) (Variables|Default|GetInitPos) _index) "0, 0, 0" "1.000000,1.000000,1.000000")))
    (Rendering|Components|Light|SetLightColor _returnvalue (Class|KismetMathLibrary|HSVtoRGBLinear (Utilities|Struct|MakeLinearColor (Math|Random|RandomFloatinRangefromStream (Variables|Default|GetStream) 0.0 3.6e+02) 1.0 1.0 1.0)) true)
    (Class|PointLightComponent|SetSourceRadius _returnvalue (Math|Random|RandomFloatinRangefromStream (Variables|Default|GetStream) (.x _lightsradius) (.y _lightsradius)))
    (Rendering|Components|Light|SetIntensity _returnvalue (Math|Random|RandomFloatinRangefromStream (Variables|Default|GetStream) (.x _lightsintensity) (.y _lightsintensity)))
    (Utilities|Array|Add (Variables|Default|GetLights) _returnvalue)
    (Components|InstancedStaticMesh|AddInstance (Variables|Default|GetISM_Lights) (Math|Transform|MakeTransform (Utilities|Array|Get(acopy) (Variables|Default|GetInitPos) _index) "0, 0, 0" (Variables|Default|GetScale)) false)))

(event EventBeginPlay
  (Actor|Tick|SetActorTickEnabled (Variables|Default|GetAnimate)))

(event Collision|EventActorBeginOverlap
  (params (OtherActor :type Actor%20Object%20Reference)))

(event EventTick
  (params (DeltaSeconds :type Float%20%28single-precision%29))
  (for _index (range 0 (- (Utilities|Array|Length (Variables|Default|GetLights)) 1))
    (Transformation|SetRelativeTransform (Utilities|Array|Get(acopy) (Variables|Default|GetLights) _index) (Math|Transform|MakeTransform (Math|Vector|MakeVector (+ (.x (Utilities|Array|Get(acopy) (Variables|Default|GetInitPos) _index)) (* (Math|Trig|Sin(Radians) (* (Utilities|Time|GetGameTimeinSeconds) (- (Math|Integer|%(Integer) _index 5) 5))) 5e+01)) (+ (.y (Utilities|Array|Get(acopy) (Variables|Default|GetInitPos) _index)) (* (Math|Trig|Cos(Radians) (* (Utilities|Time|GetGameTimeinSeconds) (- (Math|Integer|%(Integer) _index 5) 5))) 5e+01)) (.z (Utilities|Array|Get(acopy) (Variables|Default|GetInitPos) _index))) "0, 0, 0" "1.000000,1.000000,1.000000") true false)
    (Components|InstancedStaticMesh|UpdateInstanceTransform (Variables|Default|GetISM_Lights) _index (Math|Transform|MakeTransform (Math|Vector|MakeVector (+ (.x (Utilities|Array|Get(acopy) (Variables|Default|GetInitPos) _index)) (* (Math|Trig|Sin(Radians) (* (Utilities|Time|GetGameTimeinSeconds) (- (Math|Integer|%(Integer) _index 5) 5))) 5e+01)) (+ (.y (Utilities|Array|Get(acopy) (Variables|Default|GetInitPos) _index)) (* (Math|Trig|Cos(Radians) (* (Utilities|Time|GetGameTimeinSeconds) (- (Math|Integer|%(Integer) _index 5) 5))) 5e+01)) (.z (Utilities|Array|Get(acopy) (Variables|Default|GetInitPos) _index))) "0, 0, 0" (Variables|Default|GetScale)) false true false)))

(fn ConstructionScript
  (CallFunction|GenerateLights))